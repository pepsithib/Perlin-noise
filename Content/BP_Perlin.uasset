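; Actor Blueprint that works as a one-shot 2D Perlin noise texture generator.
; On BeginPlay it sets the seed, either randomized or taken from the Seed variable depending on RandSeed.
; It then calls GeneratePerlinNoise2D with the Size variable as texture dimensions and the seed as the asset path.
; The game quits immediately afterward, so each play session performs a single generation run.
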(event `self.ReceiveBeginPlay`
  (if (`self.RandSeed`)
    (bind _output_get (set `self.Seed` (`KismetMathLibrary.RandomInteger` 999999)))
    (`self.SetSeed` _output_get)
    (else
      (`self.SetSeed` (`self.Seed`))))
  (`self.GeneratePerlinNoise2D` (`KismetMathLibrary.Conv_VectorToVector2D` (`self.Size`)) (`KismetStringLibrary.Conv_IntToString` (`self.Seed`)))
  (`KismetSystemLibrary.QuitGame` null "Quit"))

(fn `UserConstructionScript`)